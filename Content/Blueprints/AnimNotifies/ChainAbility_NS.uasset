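; Anim notify state that marks an ability chain window on the animated owner's PlayerCombatComponent.
; On begin it sets the component to its configured ChainState, and on end it resets that state to None.
; The tick does nothing, as its logic to retry a buffered action through the controller's PlayerInputComponent is disconnected and never runs.
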(fn ReceivedNotifyBegin
  (params (MeshComp :type Skeletal%20Mesh%20Component%20Object%20Reference) (Animation :type Anim%20Sequence%20Base%20Object%20Reference) (TotalDuration :type Float%20%28single-precision%29))
  (bind _returnvalue (Components|GetOwner MeshComp))
  (bind _returnvalue_2 (Actor|GetComponentbyClass _returnvalue "/Script/Ascension.PlayerCombatComponent"))
  (Utilities|IsValid _returnvalue_2
    (:Is%20Valid
      (Class|PlayerCombatComponent|SetChainState _returnvalue_2 (Variables|Default|GetChainState))
      (return true))
    (:Is%20Not%20Valid
      (return false))))

(fn ReceivedNotifyEnd
  (params (MeshComp :type Skeletal%20Mesh%20Component%20Object%20Reference) (Animation :type Anim%20Sequence%20Base%20Object%20Reference))
  (bind _returnvalue (Components|GetOwner MeshComp))
  (bind _returnvalue_2 (Actor|GetComponentbyClass _returnvalue "/Script/Ascension.PlayerCombatComponent"))
  (Utilities|IsValid _returnvalue_2
    (:Is%20Valid
      (Class|PlayerCombatComponent|SetChainState _returnvalue_2 "ECS_None")
      (return true))
    (:Is%20Not%20Valid
      (return false))))

(fn ReceivedNotifyTick
  (params (MeshComp :type Skeletal%20Mesh%20Component%20Object%20Reference) (Animation :type Anim%20Sequence%20Base%20Object%20Reference) (FrameDeltaTime :type Float%20%28single-precision%29))
  (return true))