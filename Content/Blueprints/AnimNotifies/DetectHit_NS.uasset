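; Anim notify state that opens a hit-detection window during an attack animation.
; It looks up the AttackComponent on the mesh's owner and calls DetectHit on every notify tick.
; It clears that component's damaged actors list when the window begins and again when it ends.
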(fn ReceivedNotifyBegin
  (params (MeshComp :type Skeletal%20Mesh%20Component%20Object%20Reference) (Animation :type Anim%20Sequence%20Base%20Object%20Reference) (TotalDuration :type Float%20%28single-precision%29))
  (bind _returnvalue (Components|GetOwner MeshComp))
  (bind _returnvalue_2 (Actor|GetComponentbyClass _returnvalue "/Script/Ascension.AttackComponent"))
  (Utilities|IsValid _returnvalue_2
    (:Is%20Valid
      (Class|AttackComponent|ClearDamagedActors _returnvalue_2)
      (return true))))

(fn ReceivedNotifyTick
  (params (MeshComp :type Skeletal%20Mesh%20Component%20Object%20Reference) (Animation :type Anim%20Sequence%20Base%20Object%20Reference) (FrameDeltaTime :type Float%20%28single-precision%29))
  (bind _returnvalue (Components|GetOwner MeshComp))
  (bind _returnvalue_2 (Actor|GetComponentbyClass _returnvalue "/Script/Ascension.AttackComponent"))
  (Utilities|IsValid _returnvalue_2
    (:Is%20Valid
      (Class|AttackComponent|DetectHit _returnvalue_2)
      (return false))))

(fn ReceivedNotifyEnd
  (params (MeshComp :type Skeletal%20Mesh%20Component%20Object%20Reference) (Animation :type Anim%20Sequence%20Base%20Object%20Reference))
  (bind _returnvalue (Components|GetOwner MeshComp))
  (bind _returnvalue_2 (Actor|GetComponentbyClass _returnvalue "/Script/Ascension.AttackComponent"))
  (Utilities|IsValid _returnvalue_2
    (:Is%20Valid
      (Class|AttackComponent|ClearDamagedActors _returnvalue_2)
      (return false))))