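; Goblin enemy character that layers melee combat, hit reactions, death and a health bar onto its parent class.
; Hits apply attack effects and interrupt active attacks, then play an impact montage or kill and destroy the goblin after a delay.
; AI perception enters combat on sensing a player-tagged actor, while Tick mirrors PauseAI into the Blackboard.
; The construction script assigns the sword hitbox and light attack ability; footstep sound is an empty TODO.
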(event OnTargetPerceptionUpdated(AIPerception)
  (params (Actor :type Actor%20Object%20Reference) (Stimulus :type AI%20Stimulus%20Structure))
  ;[1 1 1] AI Perception
  (bind _returnvalue (Class|Goblin|IsDead))
  (if (not _returnvalue)
    (if (.bSuccessfullySensed (Utilities|Struct|BreakAIStimulus Stimulus))
      (if (Actor|ActorHasTag Actor "Player")
        (Class|Goblin|EnterCombat Actor)))))

(event Custom|Slash%20Sound
  ;[1 1 1] Audio
  ;;[1 1 1] Sword Slash Sound
  (Audio|PlaySoundatLocation "/Game/Assets/Audio/SlashCue.SlashCue" (Transformation|GetWorldLocation (Variables|Default|GetSlashLoc)) "0, 0, 0" 1.0 1.0 0.0 0 0 0))

(event EventBeginPlay
  ;[1 1 1] Setup Health Bar
  (bind _ashealth_bar (Utilities|Casting|CastToHealthBar (UserInterface|GetUserWidgetObject (Variables|Default|GetHealthBar))))
  (Variables|/Game/Blueprints/Widgets/HealthBar.HealthBar_C|SetOwningActor _ashealth_bar self))

(event EventTick
  (params (DeltaSeconds :type Float%20%28single-precision%29))
  ;[1 1 1] Enabling/Disabling AI
  (AI|Components|Blackboard|SetValueasBool (AI|GetBlackboard (Pawn|GetController)) (Variables|Default|GetPauseAIBlackboardKeyName) (Variables|Default|GetPauseAI)))

(event EventFootstepSound
  ;[1 1 1] Audio
  ;;[1 1 1] Footsounds (TODO: Implement This)
)

(event EventShowHitVisuals
  ;[1 1 1] Blueprint Overrides
  ;;[1 1 1] Show Hit Visuals
  (bind _returnvalue (Effects|SpawnEmitteratLocation "/Game/Assets/Packs/StarterContent/Particles/P_HitEffect.P_HitEffect" (Transformation|GetWorldLocation (Variables|Default|GetHitEffectLocation))))
  (Transformation|SetRelativeScale3D _returnvalue "0.700000,0.700000,0.700000")
  (Audio|PlaySoundatLocation "/Game/Assets/Audio/HitEffectCue.HitEffectCue" (Transformation|GetWorldLocation (Variables|Default|GetHitEffectLocation)) "0, 0, 0" 1.0 1.0 0.0 0 0 0))

(event EventKillActor
  ;[1 1 1] Blueprint Overrides
  ;;[1 1 1] Kill Actor
  (|CallParentFunction)
  (Animation|PlayAnimMontage "/Game/Blueprints/Enemies/Goblin/AnimMontages/fallback_death.fallback_death" 1.0 "None")
  (Collision|SetCollisionEnabled (Variables|Default|GetCapsuleComponent) "NoCollision"))

(event EventShowHealthBar
  ;[1 1 1] Interface Overrides
  ;;[1 1 1] Show/Hide Health Bar
  (Development|SetHiddeninGame (Variables|Default|GetHealthBar) false false))

(event EventHideHealthBar
  ;[1 1 1] Interface Overrides
  ;;[1 1 1] Show/Hide Health Bar
  (Development|SetHiddeninGame (Variables|Default|GetHealthBar) true false))

(event EventApplyHitEffect
  (params (SourceActor :type Actor%20Object%20Reference) (Damage :type Float%20%28single-precision%29) (HitEffect :type EHitEffect%20Enum :default "HE_PushBack") (AttackEffect :type Attack%20Effect%20Structure))
  ;[1 1 1] Interface Overrides
  ;;[1 1 1] Applying Attack Effects
  (if (not (Variables|Default|GetDead))
    (Class|Goblin|ShowHitVisuals)
    (Class|Goblin|ApplyAttackEffects SourceActor Damage HitEffect AttackEffect)
    (if (Utilities|Enum|Equal(Enum) (Variables|Default|GetActionState) "ES_Attacking")
      (Class|Goblin|ResetAttack)
      (Default|CallOnAttackComplete (Variables|Default|GetAttackComponent) false))
    (bind _returnvalue (Class|Goblin|CheckDead))
    (if _returnvalue
      (Class|Goblin|KillActor)
      (Utilities|FlowControl|Delay 5.0)
      (Actor|DestroyActor)
      (else
        (Animation|PlayAnimMontage "/Game/Blueprints/Enemies/Goblin/AnimMontages/GS_Impact.GS_Impact" 1.5 "None")
        (Default|CallOnHit)))))

(event EventAttackComplete
  ;[1 1 1] Attack Complete Broadcast
  (Default|CallOnAttackComplete (Variables|Default|GetAttackComponent) true))

(fn ConstructionScript
  (Variables|/Script/Ascension.AttackComponent|SetAttackHitBox (Variables|Default|GetAttackComponent) (Variables|Default|GetSwordHitBox))
  (Class|GameAbilitySystemComponent|ClearAbilities (Variables|Default|GetAbilitySystemComponent))
  (CallFunction|AddAbility "/Game/Blueprints/Enemies/Goblin/Abilities/Goblin_Light01.Goblin_Light01_C"))

(fn AddAbility
  (params (Class :type Ability%20Class%20Reference) (AbilityName :type String))
  (Class|GameAbilitySystemComponent|AddAbility (Variables|Default|GetAbilitySystemComponent) AbilityName Class))